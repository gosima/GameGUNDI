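; Choppable tree actor that shatters its Destructible mesh when chopped with the top-down character in range, then shrinks away.
; Collision overlaps set the character's InRangeOfTree flag, which ChopDownTree checks before applying axe damage.
; After a delay, a Tick gate opens to scale the tree down until destroyed.
; A second gate, opened by WiggleTree, steps pitch back, forward and back to upright, then resets.
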(event OnComponentBeginOverlap(Collision)
  (params (OtherActor :type Actor%20Object%20Reference) (OtherComp :type Primitive%20Component%20Object%20Reference) (OtherBodyIndex :type Integer) (bFromSweep :type Boolean) (SweepResult :type Hit%20Result%20Structure%20%28by%20ref%29))
  (bind _astop_down_character (Utilities|Casting|CastToTopDownCharacter OtherActor))
  (Variables|Default|SetOverlappedTDCRef _astop_down_character)
  (Variables|/Game/Blueprints/Character/TopDownCharacter.TopDownCharacter_C|SetInRangeOfTree (Variables|Default|GetOverlappedTDCRef) true))

(event OnComponentEndOverlap(Collision)
  (params (OtherActor :type Actor%20Object%20Reference) (OtherComp :type Primitive%20Component%20Object%20Reference) (OtherBodyIndex :type Integer))
  (Variables|/Game/Blueprints/Character/TopDownCharacter.TopDownCharacter_C|SetInRangeOfTree (Variables|Default|GetOverlappedTDCRef) false))

(event Custom|DestroySelf
  ;[1 1 1] Destroy Self
  (Variables|/Game/Blueprints/Character/TopDownCharacter.TopDownCharacter_C|SetInRangeOfTree (Variables|Default|GetOverlappedTDCRef) false)
  (Utilities|FlowControl|Delay 5.0)
  (Utilities|FlowControl|Gate true) ; enters at Open
)

(event Custom|DoneWiggling
  ;[1 1 1] Wiggle Effect
  (Utilities|FlowControl|Gate true) ; enters at Close
)

(event Custom|WiggleTree
  ;[1 1 1] Wiggle Effect
  (Utilities|FlowControl|Gate true) ; enters at Open
)

(event Custom|ChopDownTree
  (params (AxeDamage :type Integer))
  (bind _destructible (Variables|Default|GetDestructible))
  (bind _returnvalue (Transformation|GetWorldLocation _destructible))
  ;[1 1 1] Chop down tree
  (if (Variables|/Game/Blueprints/Character/TopDownCharacter.TopDownCharacter_C|GetInRangeOfTree (Variables|Default|GetOverlappedTDCRef))
    (Game|Damage|ApplyDamage (Variables|Default|GetDestructible) (Math|Conversions|ToFloat(Integer) AxeDamage) _returnvalue _returnvalue 0.0)
    (CallFunction|DestroySelf)))

(event EventTick
  (params (DeltaSeconds :type Float%20%28single-precision%29))
  (Utilities|FlowControl|Sequence
    (:then_0
      ;[1 1 1] Destroy Self
      (Utilities|FlowControl|Gate true
        (:Exit
          (if (< (.X (Math|Vector|BreakVector (Variables|/Script/Engine.SceneComponent|GetRelativeScale3D (Variables|Default|GetDestructible)))) 0.0)
            (Actor|DestroyActor)
            (else
              (Transformation|SetActorScale3D (- (Variables|/Script/Engine.SceneComponent|GetRelativeScale3D (Variables|Default|GetDestructible)) "0.010000,0.010000,0.010000")))))))
    (:then_1
      ;[1 1 1] Wiggle Effect
      (Utilities|FlowControl|Gate true
        (:Exit
          (if (not (Variables|Wiggle|GetBackDone))
            (Utilities|LeanBack)
            (elif (not (Variables|Wiggle|GetFrontDone))
              (Utilities|LeanForward)
              (elif (not (Variables|Wiggle|GetDone))
                (Utilities|BacktoNormal)
                (else
                  (Utilities|Reset))))))))))

(fn ConstructionScript)